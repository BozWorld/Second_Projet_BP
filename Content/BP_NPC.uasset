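; BP_NPC is an interactable NPC that runs a placeholder dialogue with a four-way choice whose branches are empty.
; Overlapping its collision binds NPC_Interact to the player character's interact event and shows a prompt widget; leaving undoes both.
; Each interaction hides the prompt and sets a line-skip flag, while a DoOnce, never reset here, creates the dialogue widget and feeds it lines and choices.
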(event OnComponentBeginOverlap(NPC_Collision)
  (params (OverlappedComponent :type Primitive%20Component%20Object%20Reference) (OtherActor :type Actor%20Object%20Reference) (OtherComp :type Primitive%20Component%20Object%20Reference) (OtherBodyIndex :type Integer) (bFromSweep :type Boolean) (SweepResult :type Hit%20Result%20Structure%20%28by%20ref%29))
  (bind _asbp_third_person_character (Utilities|Casting|CastToBP_ThirdPersonCharacter OtherActor))
  (EventDispatchers|BindEventtoInteract _asbp_third_person_character (delegate Custom|NPC_Interact))
  (Rendering|SetVisibility (Variables|Default|GetInteract_Widget) true false))

(event OnComponentEndOverlap(NPC_Collision)
  (params (OverlappedComponent :type Primitive%20Component%20Object%20Reference) (OtherActor :type Actor%20Object%20Reference) (OtherComp :type Primitive%20Component%20Object%20Reference) (OtherBodyIndex :type Integer))
  (bind _asbp_third_person_character (Utilities|Casting|CastToBP_ThirdPersonCharacter OtherActor))
  (EventDispatchers|UnbindEventfromInteract _asbp_third_person_character (delegate Custom|NPC_Interact))
  (Rendering|SetVisibility (Variables|Default|GetInteract_Widget) false false))

(event Custom|NPC_Interact
  (Rendering|SetVisibility (Variables|Default|GetInteract_Widget) false false)
  (Variables|Default|SetSkipLIne true)
  (Utilities|FlowControl|DoOnce false
    (:Completed
      (bind _returnvalue (UserInterface|CreateWidget "/Game/dialogue/WBP_dialogue.WBP_dialogue_C"))
      (UserInterface|Viewport|AddtoViewport _returnvalue 0)
      (Variables|Default|SetDialogue%20Widget _returnvalue)
      (Utilities|AddDialogueLine self "wawawawa")
      (Utilities|AddDialogueLine self "ahhhhhhhhhhhh")
      (Utilities|AddChoice self "a" "b" "c" "d"
        (:choix_1
          _)
        (:choix_2
          _)
        (:choix_3
          _)
        (:choix_4
          _))
      (Development|PrintString "Hello")
      (Widget|RemovefromParent (Variables|Default|GetDialogue%20Widget)))))

(fn ConstructionScript)