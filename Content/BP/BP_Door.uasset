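; BP_Door is an interactable door that the third-person character can open by playing an animation sequence.
; Overlapping its collision while the character's CanOpen flag is set binds OpenDoor to the character's Interact event dispatcher and shows a prompt widget.
; Leaving the collision unbinds it and hides the prompt.
; OpenDoor plays the DoorAnimator sequence player and hides the prompt.
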(event OnComponentBeginOverlap(DoorCollision)
  (params (OverlappedComponent :type Primitive%20Component%20Object%20Reference) (OtherActor :type Actor%20Object%20Reference) (OtherComp :type Primitive%20Component%20Object%20Reference) (OtherBodyIndex :type Integer) (bFromSweep :type Boolean) (SweepResult :type Hit%20Result%20Structure%20%28by%20ref%29))
  (bind _asbp_third_person_character (Utilities|Casting|CastToBP_ThirdPersonCharacter OtherActor))
  (if (Variables|/Game/ThirdPerson/Blueprints/BP_ThirdPersonCharacter.BP_ThirdPersonCharacter_C|GetcanOpen _asbp_third_person_character)
    (EventDispatchers|BindEventtoInteract _asbp_third_person_character (delegate Custom|OpenDoor))
    (Rendering|SetVisibility (Variables|Default|GetInteract_Widget) true false)))

(event OnComponentEndOverlap(DoorCollision)
  (params (OverlappedComponent :type Primitive%20Component%20Object%20Reference) (OtherActor :type Actor%20Object%20Reference) (OtherComp :type Primitive%20Component%20Object%20Reference) (OtherBodyIndex :type Integer))
  (bind _asbp_third_person_character (Utilities|Casting|CastToBP_ThirdPersonCharacter OtherActor))
  (EventDispatchers|UnbindEventfromInteract _asbp_third_person_character (delegate Custom|OpenDoor))
  (Rendering|SetVisibility (Variables|Default|GetInteract_Widget) false false))

(event Custom|OpenDoor
  (Sequencer|Player|Play (Variables|/Script/ActorSequence.ActorSequenceComponent|GetSequencePlayer (Variables|Default|GetDoorAnimator)) :!class /Script/MovieScene.MovieSceneSequencePlayer)
  (Rendering|SetVisibility (Variables|Default|GetInteract_Widget) false false))

(fn ConstructionScript)